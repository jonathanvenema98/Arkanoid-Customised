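; HUD that doubles as the game manager for a three-level brick breaker, drawing level, lives, start and win text.
; Bricks spawn at TargetPoints tagged per level, with random health after the first level.
; Brick and life events update counters that drive level advance, win and game over, clearing leftover powerups on either ending.
; It resets the ball and rocket paddle between rounds and relaunches them after a delay.
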(event Custom|SpawnBricks
  (if (== (Variables|Default|GetLevel) 1)
    (bind _outactors (Actor|GetAllActorsOfClasswithTag "/Script/Engine.TargetPoint" "lvl1"))
    (for _array_element _outactors
      (bind _returnvalue (Game|SpawnActorfromClass "/Game/Blueprints/Actor_Brick.Actor_Brick_C" (Math|Transform|MakeTransform (Transformation|GetActorLocation _array_element) "0, 0, 0" "1,1,1") "Undefined" 0 0))
      (bind _result (Math|Integer|IncrementInt (Variables|Default|GetBricksLeftInLevel))
        (:%20%20
          (Variables|Default|SetBricksLeftInLevel _result)
          (if (== (Variables|Default|GetLevel) 1)
            (Default|SetHealth _returnvalue 1)
            (else
              (Default|SetHealth _returnvalue (Math|Random|RandomIntegerinRange 1 3)))))))
    (elif (== (Variables|Default|GetLevel) 2)
      (bind _outactors_2 (Actor|GetAllActorsOfClasswithTag "/Script/Engine.TargetPoint" "lvl2"))
      (for _array_element_2 _outactors_2
        (bind _returnvalue_2 (Game|SpawnActorfromClass "/Game/Blueprints/Actor_Brick.Actor_Brick_C" (Math|Transform|MakeTransform (Transformation|GetActorLocation _array_element_2) "0, 0, 0" "1,1,1") "Undefined" 0 0))
        (bind _result_2 (Math|Integer|IncrementInt (Variables|Default|GetBricksLeftInLevel))
          (:%20%20
            (Variables|Default|SetBricksLeftInLevel _result_2)
            (if (== (Variables|Default|GetLevel) 1)
              (Default|SetHealth _returnvalue_2 1)
              (else
                (Default|SetHealth _returnvalue_2 (Math|Random|RandomIntegerinRange 1 3)))))))
      (else
        (bind _outactors_3 (Actor|GetAllActorsOfClasswithTag "/Script/Engine.TargetPoint" "lvl3"))
        (for _array_element_3 _outactors_3
          (bind _returnvalue_3 (Game|SpawnActorfromClass "/Game/Blueprints/Actor_Brick.Actor_Brick_C" (Math|Transform|MakeTransform (Transformation|GetActorLocation _array_element_3) "0, 0, 0" "1,1,1") "Undefined" 0 0))
          (bind _result_3 (Math|Integer|IncrementInt (Variables|Default|GetBricksLeftInLevel))
            (:%20%20
              (Variables|Default|SetBricksLeftInLevel _result_3)
              (if (== (Variables|Default|GetLevel) 1)
                (Default|SetHealth _returnvalue_3 1)
                (else
                  (Default|SetHealth _returnvalue_3 (Math|Random|RandomIntegerinRange 1 3)))))))))))

(event Custom|BrickDestroyed
  (Math|Integer|DecrementInt (Variables|Default|GetBricksLeftInLevel)
    (:%20%20
      (if (== (Variables|Default|GetBricksLeftInLevel) 0)
        (bind _result (Math|Integer|IncrementInt (Variables|Default|GetLevel))
          (:%20%20
            (bind _output_get (Variables|Default|SetLevel _result))
            (if (== _output_get 4)
              (Variables|Default|SetGameWon true)
              (Variables|Default|SetGameOver true)
              (bind _outactors (Actor|GetAllActorswithTag "Powerup"))
              (for _array_element _outactors
                (Actor|DestroyActor _array_element)
                (CallFunction|ResetNumberOfLives)
                (CallFunction|SpawnBricks)
                (CallFunction|ResetScene)
                (CallFunction|ResetLevel))
              (else
                (CallFunction|ResetScene)
                (CallFunction|SpawnBricks)
                (CallFunction|StartBallandPaddle)))))))))

(event Custom|StartBallAndPaddle
  (Utilities|FlowControl|Delay (Variables|Default|GetDelayBeforeStart))
  (Default|EnablePaddleMovement (Variables|Default|GetRocketPlatform))
  (Default|SetInitialDirection (Variables|Default|GetBall)))

(event Custom|ResetScene
  (Default|ZeroInitialDirection (Variables|Default|GetBall))
  (Default|ResetLocation (Variables|Default|GetBall))
  (Default|ResetLocationDisableInput (Variables|Default|GetRocketPlatform)))

(event Custom|EnterPressed
  (if (Variables|Default|GetGameWon)
    (CallFunction|ResetScene)
    (CallFunction|ResetNumberOfLives)
    (CallFunction|SpawnBricks))
  (if (Variables|Default|GetGameOver)
    (Variables|Default|SetGameOver false)
    (Variables|Default|SetGameWon false)
    (CallFunction|StartBallandPaddle)))

(event Custom|ResetNumberOfLives
  (Variables|Default|SetLives (Variables|Default|GetDefaultNumberOfLives)))

(event Custom|DecrementLives
  (bind _result (Math|Integer|DecrementInt (Variables|Default|GetLives))
    (:%20%20
      (bind _output_get (Variables|Default|SetLives _result))
      (if (<= _output_get 0)
        (Variables|Default|SetGameOver true)
        (bind _outactors (Actor|GetAllActorsOfClass "/Game/Blueprints/Actor_Brick.Actor_Brick_C"))
        (for _array_element _outactors
          (Actor|DestroyActor _array_element))
        (bind _outactors_2 (Actor|GetAllActorswithTag "Powerup"))
        (for _array_element_2 _outactors_2
          (Actor|DestroyActor _array_element_2))
        (Variables|Default|SetBricksLeftInLevel 0)
        (CallFunction|ResetNumberOfLives)
        (CallFunction|ResetLevel)
        (CallFunction|SpawnBricks))
      (CallFunction|ResetScene)
      (if (not (Variables|Default|GetGameOver))
        (CallFunction|StartBallandPaddle)))))

(event Custom|ExtraLifePowerupConsumed
  (bind _result (Math|Integer|IncrementInt (Variables|Default|GetLives))
    (:%20%20
      (Variables|Default|SetLives _result))))

(event Custom|ResetLevel
  (Variables|Default|SetLevel 1))

(event EventBeginPlay
  (bind _outactors (Actor|GetAllActorsOfClass "/Game/Blueprints/Actor_RocketPlatform.Actor_RocketPlatform_C"))
  (Variables|Default|SetRocketPlatform (Utilities|Array|Get(acopy) _outactors))
  (bind _outactors_2 (Actor|GetAllActorsOfClass "/Game/Blueprints/Character_Ball2.Character_Ball2_C"))
  (Variables|Default|SetBall (Utilities|Array|Get(acopy) _outactors_2))
  (Variables|Default|SetGameOver true)
  (Variables|Default|SetGameWon false)
  (CallFunction|ResetNumberOfLives)
  (CallFunction|SpawnBricks))

(event Collision|EventActorBeginOverlap
  (params (OtherActor :type Actor%20Object%20Reference)))

(event EventDrawHUD
  (params (SizeX :type Integer) (SizeY :type Integer))
  (if (Variables|Default|GetGameWon)
    (HUD|DrawText "Congratulations! 
      You Won 
 
  Press Enter to 
     play again" "(R=0.947307,G=0.982251,B=1.000000,A=1.000000)" 8e+01 2.2e+02 0 5.0 false)
    (elif (Variables|Default|GetGameOver)
      (HUD|DrawText "Press Enter  
   to Start" "(R=0.943905,G=0.979617,B=1.000000,A=1.000000)" 8e+01 2.2e+02 0 4.0 false)
      (else
        (HUD|DrawText (Utilities|String|BuildString(Integer) "" "Level: " (Variables|Default|GetLevel)) "(R=0.000000,G=0.796875,B=0.018107,A=1.000000)" 1.5e+02 128.0 0 3.0 false)
        (HUD|DrawText (Utilities|String|BuildString(Integer) "" "Lives: " (Variables|Default|GetLives)) "(R=0.000000,G=0.813084,B=1.000000,A=1.000000)" 1.5e+02 256.0 0 3.0 false)))))

(fn ConstructionScript)