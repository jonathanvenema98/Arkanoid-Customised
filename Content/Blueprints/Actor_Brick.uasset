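; Breakout-style brick actor that wears down with each hit and can drop a bonus capsule when destroyed.
; Health is set through SetHealth and selects the clean, marked or heavily worn sprite.
; CollisionDetected decrements Health; at zero or below it destroys the brick and notifies GameManagerHUD.
; On level 3 only, chained independent random rolls may first spawn an acceleration, deceleration, extra-life or wider-platform capsule.
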(event Custom|SetHealth
  (params (NumberOfLives :type Integer))
  (Variables|Default|SetHealth NumberOfLives)
  (CallFunction|UpdateSprite))

(event Custom|UpdateSprite
  (bind _sprite_brickwithsignificantwear (Variables|Default|GetSprite_BrickWithSignificantWear))
  (bind _health (Variables|Default|GetHealth))
  (if (== _health 1)
    (Rendering|Components|Sprite|SetSprite _sprite_brickwithsignificantwear "/Game/Sprites/Sprite_BrickWithSignificantWear.Sprite_BrickWithSignificantWear")
    (elif (== _health 2)
      (Rendering|Components|Sprite|SetSprite _sprite_brickwithsignificantwear "/Game/Sprites/Sprite_Brick_with_marks.Sprite_Brick_with_marks")
      (else
        (Rendering|Components|Sprite|SetSprite _sprite_brickwithsignificantwear "/Game/Sprites/Sprite_Brick_clean.Sprite_Brick_clean")))))

(event EventBeginPlay)

(event Collision|EventActorBeginOverlap
  (params (OtherActor :type Actor%20Object%20Reference)))

(event EventTick
  (params (DeltaSeconds :type Float%20%28single-precision%29)))

(fn ConstructionScript)

(fn CollisionDetected
  (bind _returnvalue (Math|Random|RandomIntegerinRange 1 20))
  (bind _returnvalue_2 (Transformation|GetActorTransform))
  ;[1 1 1] If health is not 0, change sprite to represent updated health (ie more cracks)
  (bind _result (Math|Integer|DecrementInt (Variables|Default|GetHealth))
    (:%20%20
      (Math|Integer|CompareInt _result
        (:>
          (CallFunction|UpdateSprite))
        (:==
          ;[1 1 1] Only spawn bonuses on level 3
          (bind _returnvalue_3 (Actor|GetActorOfClass "/Game/Blueprints/GameManagerHUD.GameManagerHUD_C" :!label _label))
          (if (== (Variables|/Game/Blueprints/GameManagerHUD.GameManagerHUD_C|GetLevel _returnvalue_3) 3)
            ;[1 1 1] Spawn a bonus at the brick location
            (if (== _returnvalue 1)
              (Game|SpawnActorfromClass "/Game/Blueprints/Actor_AccelerationCapsule.Actor_AccelerationCapsule_C" _returnvalue_2 "AlwaysSpawn" 0 0)
              (elif (== _returnvalue 2)
                (Game|SpawnActorfromClass "/Game/Blueprints/Actor_DecelerateCapsule.Actor_DecelerateCapsule_C" _returnvalue_2 "AlwaysSpawn" 0 0)
                (elif (== _returnvalue 3)
                  (Game|SpawnActorfromClass "/Game/Blueprints/Actor_ExtraLifeCapsule.Actor_ExtraLifeCapsule_C" _returnvalue_2 "AlwaysSpawn" 0 0)
                  (elif (== _returnvalue 4)
                    (Game|SpawnActorfromClass "/Game/Blueprints/Actor_WiderPlatformCapsule.Actor_WiderPlatformCapsule_C" _returnvalue_2 "AlwaysSpawn" 0 0))))))
          ;[1 1 1] Destroy the actor, update the GameManagerHUD to reflect the decrease in brick numbers
          (Actor|DestroyActor)
          (bind _outactors (Actor|GetAllActorsOfClass "/Game/Blueprints/GameManagerHUD.GameManagerHUD_C"))
          (Default|BrickDestroyed (Utilities|Array|Get(acopy) _outactors)))
        (:<
          (goto _label))))))